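; EnemySpawn is a room actor that starts a combat encounter as soon as play begins.
; It generates and runs a "ShunnedHouse" combat event, then spawns that event's enemy actor at its own location.
; It disables player movement and rotation, blends the camera to the enemy, and opens the DungeonHUD deck with UI-only mouse input.
; The enemy data is passed to the Player last, after the HUD is created.
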(event EventBeginPlay
  (bind _returnvalue (Game|GetPlayerController 0))
  (bind _event (CallFunction|GenerateCombat "ShunnedHouse"))
  (Variables|Default|SetEvent _event)
  (CallFunction|RunEvent (Variables|Default|GetEvent))
  (Default|ToggleMovementRotation (.AsPlayer (Utilities|Casting|CastToPlayer (Game|GetPlayerCharacter 0))) false false)
  (bind _returnvalue_2 (Game|SpawnActorfromClass (.EnemyActor (Utilities|Struct|BreakST_Enemy (.EnemyData (Utilities|Struct|BreakST_Event (Variables|Default|GetEvent))))) (Math|Transform|MakeTransform (Transformation|GetActorLocation self) "0,-90.000000, 0") "Undefined" 0 0))
  (Game|Player|SetViewTargetwithBlend (Game|GetPlayerController 0) _returnvalue_2 2.0 "VTBlend_Linear" 0.0 false)
  (bind _returnvalue_3 (UserInterface|CreateWidget "/Game/DarkMemoireProject/UMG/HUD/DungeonHUD.DungeonHUD_C"))
  (UserInterface|Viewport|AddtoViewport _returnvalue_3 0)
  (Default|ShowDeck _returnvalue_3)
  (Input|SetInputModeUIOnly _returnvalue 0 "DoNotLock")
  (Variables|/Script/Engine.PlayerController|SetbShowMouseCursor _returnvalue true)
  (Variables|/Game/DarkMemoireProject/Blueprints/PlayerCharacter/Player.Player_C|SetEnemyData (.AsPlayer (Utilities|Casting|CastToPlayer (Game|GetPlayerCharacter 0))) (.EnemyData (Utilities|Struct|BreakST_Event (Variables|Default|GetEvent)))))

(fn ConstructionScript)