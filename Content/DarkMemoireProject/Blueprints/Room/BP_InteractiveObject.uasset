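; Interactive room object that shows a text prompt to an overlapping player while it has a ready event to trigger.
; SetEvent assigns an event and arms the object, which counts as interactable only while armed and that event is ready.
; Overlap begin caches the player and shows the text, and that player's exit hides it if still interactable.
; Activation disarms the object and dispatches a player-interaction notification carrying the event.
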(event Custom|OnObjectActivated
  (Variables|Default|SetIsActivate false)
  (Default|CallDispatchPlayerInteractedwithObject (Variables|Default|GetEvent)))

(event EventBeginPlay
  (Rendering|SetVisibility (Variables|Default|GetTextRender) false false))

(event Collision|EventActorBeginOverlap
  (params (OtherActor :type Actor%20Object%20Reference))
  (bind _event_is_ready (CallFunction|IsInteractableObjectReady))
  (if _event_is_ready
    (bind _asplayer (Utilities|Casting|CastToPlayer OtherActor))
    (Variables|Default|SetAs%20Player _asplayer)
    (Rendering|SetVisibility (Variables|Default|GetTextRender) true false)))

(event Collision|EventActorEndOverlap
  (params (OtherActor :type Actor%20Object%20Reference))
  (bind _event_is_ready (CallFunction|IsInteractableObjectReady))
  (if (and _event_is_ready (== (Variables|Default|GetAs%20Player) OtherActor))
    (Rendering|SetVisibility (Variables|Default|GetTextRender) false false)))

(fn ConstructionScript)

(fn IsInteractableObjectReady
  (return (and (.isready (Variables|Default|GetEvent)) (Variables|Default|GetIsActivate))))

(fn SetEvent
  (params (NewEvent :type ST%20Event%20Structure))
  (Variables|Default|SetEvent NewEvent)
  (Variables|Default|SetIsActivate true))