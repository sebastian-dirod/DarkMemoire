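; BP_Door is a room door actor that shows a text prompt when the player is near and can be opened.
; It wraps a Door child actor, cached on BeginPlay with the text hidden.
; Overlap events store the player and toggle the text's visibility.
; OnOpenDoor forwards the open call to the child Door, then fires a dispatcher passing itself to notify listeners.
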(event Custom|OnOpenDoor
  (Default|OpenDoor (Variables|Default|GetDoorActor))
  (Default|CallDispatchOpenDoor self))

(event EventBeginPlay
  (bind _asdoor (Utilities|Casting|CastToDoor (Variables|/Script/Engine.ChildActorComponent|GetChildActor (Variables|Default|GetDoor))))
  (Variables|Default|SetDoorActor _asdoor)
  (Rendering|SetVisibility (Variables|Default|GetTextRender) false false))

(event Collision|EventActorBeginOverlap
  (params (OtherActor :type Actor%20Object%20Reference))
  (bind _asplayer (Utilities|Casting|CastToPlayer OtherActor))
  (Variables|Default|SetOverlappingActor _asplayer)
  (Rendering|SetVisibility (Variables|Default|GetTextRender) true false))

(event Collision|EventActorEndOverlap
  (params (OtherActor :type Actor%20Object%20Reference))
  (if (== (Variables|Default|GetOverlappingActor) OtherActor)
    (Rendering|SetVisibility (Variables|Default|GetTextRender) false false)))

(fn ConstructionScript)