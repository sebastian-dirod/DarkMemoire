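; Dungeon expedition game mode that runs room exploration, card combat, goal checks and the return to town.
; BeginPlay keeps one random room per data-table tag and seeds rooms and interactive objects with generated events.
; Doors teleport through a triangular connection matrix, which gets rewired by sanity rolls and later clock phases alongside added events and sanity drain.
; Selected cards advance the clock and resolve against enemy actions by speed, with death returning to TownScreen.
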(event Custom|HandleInteractionWithObject
  (params (ObjectEvent :type ST%20Event%20Structure))
  ;[1 1 1] Set T=0 of map, room events, interactive objects events, variables and player.
  (CallFunction|RunRoomEvent ObjectEvent))

(event Custom|HandleGoBackTown
  ;[1 1 1] Unified exit from map to TownScreen
  (bind _ascustom_game_instance (Utilities|Casting|CastToCustomGameInstance (Game|GetGameInstance)))
  (Variables|/Game/DarkMemoireProject/DataManagement/GameData/CustomGameInstance.CustomGameInstance_C|SetExpeditionAccomplished _ascustom_game_instance (Variables|Default|GetExpeditionAccomplished))
  (bind _returnvalue (UserInterface|CreateWidget "/Game/DarkMemoireProject/UMG/Generic/Fades.Fades_C"))
  (bind _output_get (Variables|Default|SetFades _returnvalue))
  (Variables|/Game/DarkMemoireProject/UMG/Generic/Fades.Fades_C|SetPlayAnim _output_get (Variables|/Game/DarkMemoireProject/UMG/Generic/Fades.Fades_C|GetFadeIn _output_get))
  (bind _output_get_2 (Variables|/Game/DarkMemoireProject/UMG/Generic/Fades.Fades_C|SetDelayAnim _output_get 2.1))
  (UserInterface|Viewport|AddtoViewport _output_get 0)
  (Utilities|FlowControl|Delay (- _output_get_2 0.2))
  (Game|OpenLevel(byName) "TownScreen"))

(event Custom|HandleOnClockUpdate
  ;[1 1 1] Update Clock, then update level
  (CallFunction|OnClockUpdate))

(event Custom|HandleOpenDoor
  (params (Door :type BP%20Door%20Object%20Reference))
  ;[1 1 1] Set T=0 of map, room events, interactive objects events, variables and player.
  ;;[1 1 1] Teleport to Next Room. Relocate Doors. Run Event in Room.
  (bind _nextdoor (CallFunction|TeleporttoNextDoor Door))
  (bind _room (CallFunction|GetDoorsRoom _nextdoor))
  (if (>= (Utilities|Array|FindItem (Variables|Default|GetRoomsVisited) _room) 0)
    _
    (else
      (Utilities|Array|Add (Variables|Default|GetRoomsVisited) _room)
      (CallFunction|CheckAllRoomsVisited)))
  (bind _sanityratio (Default|GetSanityRatio (Variables|Default|GetPlayerInstance)))
  (if (> (Math|Random|RandomFloat) _sanityratio)
    (CallFunction|RandomizeDoorsConnections))
  (if (> (Utilities|Array|Length (Variables|/Game/DarkMemoireProject/Blueprints/Room/BP_Room.BP_Room_C|GetRoomEvent _room)) 0)
    (CallFunction|RunRoomEvent (Utilities|Array|Get(acopy) (Variables|/Game/DarkMemoireProject/Blueprints/Room/BP_Room.BP_Room_C|GetRoomEvent _room)))
    (Utilities|Array|RemoveIndex (Variables|/Game/DarkMemoireProject/Blueprints/Room/BP_Room.BP_Room_C|GetRoomEvent _room))))

(event Custom|OnCardSelected
  (params (CardIndex :type Integer) (CardData :type ST%20Card%20Structure) (StackedTime :type Integer))
  ;[1 1 1] Select Card Cycle
  ;;[1 1 1] Avoid clicking another card until resolved. Clock Ticks updated by action
  (Variables|/Script/Engine.PlayerController|SetbShowMouseCursor (Game|GetPlayerController 0) false)
  (Variables|Default|SetClockTicks (+ StackedTime (Variables|Default|GetClockTicks)))
  ;[1 1 1] Combat Cycle
  (bind (_nextactiondata _nextactionspeed) (Default|GetRoundActionandSpeed (Variables|Default|GetActiveEnemy)))
  (if (> _nextactionspeed StackedTime)
    (CallFunction|ResolvePlayerAction CardData)
    (bind _returnvalue (Default|IsAlive (Variables|Default|GetActiveEnemy)))
    (if _returnvalue
      (CallFunction|ResolveEnemyAction _nextactiondata)
      (bind _isalive (Default|IsAlive (Variables|Default|GetPlayerInstance)))
      (if _isalive
        ;[1 1 1] End of CardSelected cycle. User can click on another card again if still on UI Mode
        (Variables|/Script/Engine.PlayerController|SetbShowMouseCursor (Game|GetPlayerController 0) true :!label _label)
        (else
          (CallFunction|EndCombat :!label _label_2)))
      (else
        (goto _label_2)))
    (else
      (CallFunction|ResolveEnemyAction _nextactiondata)
      (bind _isalive_2 (Default|IsAlive (Variables|Default|GetPlayerInstance)))
      (if _isalive_2
        (CallFunction|ResolvePlayerAction CardData)
        (bind _returnvalue_2 (Default|IsAlive (Variables|Default|GetActiveEnemy)))
        (if _returnvalue_2
          (goto _label)
          (else
            (goto _label_2)))
        (else
          (goto _label_2))))))

(event Custom|HandlePlayerDeath
  ;[1 1 1] Handle player has died in combat here
  (CallFunction|GoBackTown))

(event Custom|HandleCardSelected
  (params (CardIndex :type Integer) (CardData :type ST%20Card%20Structure) (StackedTime :type Integer))
  ;[1 1 1] Shortcut to Player Character
  (CallFunction|OnCardSelected CardIndex CardData StackedTime))

(event EventBeginPlay
  (Utilities|FlowControl|Sequence
    (:then_0
      ;[1 1 1] Shortcut to Player Character
      (bind _asplayer (Utilities|Casting|CastToPlayer (Game|GetPlayerCharacter 0)))
      (bind _output_get (Variables|Default|SetPlayerInstance _asplayer))
      (EventDispatchers|BindEventtoDispatchCardSelected _output_get (delegate Custom|HandleCardSelected))
      (Variables|Default|SetDungeon%20HUD (Variables|/Game/DarkMemoireProject/Blueprints/PlayerCharacter/Player.Player_C|GetDungeonHUD _output_get))
      ;;[1 1 1] 0=Walk, 1=Combat, 2=Interact
      (Variables|Default|SetCurrentGameMode 0))
    (:then_1
      ;[1 1 1] Set initial values
      (bind _returnvalue (Game|GetCurrentLevelName true))
      (bind _output_get_2 (Variables|Default|SetLevelName _returnvalue))
      (bind _returnvalue_2 (Utilities|GetDataTableRow "/Game/DarkMemoireProject/DataManagement/Tables/DB_RoomDistribution.DB_RoomDistribution" (Utilities|String|StringToName _output_get_2))
        (:then
          (Variables|Default|SetRoom%20Tags (.RoomTags (Utilities|Struct|BreakST_RoomDistribution _returnvalue_2)))
          (Variables|Default|SetRoomConnections (.RoomConnections (Utilities|Struct|BreakST_RoomDistribution _returnvalue_2)))
          (Variables|Default|SetRoomsIndexes (.RoomIndexes (Utilities|Struct|BreakST_RoomDistribution _returnvalue_2))))))
    (:then_2
      ;[1 1 1] Remove unnecessary rooms
      (for _array_element (Variables|Default|GetRoom%20Tags)
        (bind _outactors (Actor|GetAllActorsOfClasswithTag "/Game/DarkMemoireProject/Blueprints/Room/BP_Room.BP_Room_C" _array_element))
        (Utilities|Array|RemoveIndex _outactors (.OutIndex (Utilities|Array|Random _outactors)))
        (CallFunction|RemoveRoomArray _outactors)))
    (:then_3
      ;[1 1 1] Set T=0 of map, room events, interactive objects events, variables and player.
      (for _array_element_2 (Variables|Default|GetRoom%20Tags)
        (bind _outactors_2 (Actor|GetAllActorsOfClasswithTag "/Game/DarkMemoireProject/Blueprints/Room/BP_Room.BP_Room_C" _array_element_2))
        (Utilities|Map|Add (Variables|Default|GetRoomInstances) _array_element_2 (Utilities|Array|Get(acopy) _outactors_2))
        (EventDispatchers|BindEventtoDispatchOpenDoor (Utilities|Array|Get(acopy) _outactors_2) (delegate Custom|HandleOpenDoor))
        (for _array_element_3 (Variables|/Game/DarkMemoireProject/Blueprints/Room/BP_Room.BP_Room_C|GetDoors (Utilities|Array|Get(acopy) _outactors_2))
          (Utilities|Array|Add (Variables|Default|GetDoorInstances) _array_element_3)))
      (bind _outactors_3 (Actor|GetAllActorsOfClass "/Game/DarkMemoireProject/Blueprints/Room/BP_InteractiveObject.BP_InteractiveObject_C"))
      (for _array_element_4 _outactors_3
        (EventDispatchers|BindEventtoDispatchPlayerInteractedwithObject _array_element_4 (delegate Custom|HandleInteractionWithObject)))
      (CallFunction|SetPlayerStartingLocation)
      (CallFunction|AddEventstoRooms (/ (Utilities|Array|Length (Variables|Default|GetRoom%20Tags)) 2))
      (CallFunction|AddEventstoInteractiveObjects))
    (:then_4
      ;[1 1 1] Update Clock, then update level
      (Utilities|Time|SetTimerbyEvent (delegate Custom|HandleOnClockUpdate) (Variables|Default|GetSecondsToTick) true (Variables|Default|GetSecondsToTick)))
    (:then_5
      (bind _ascustom_game_instance (Utilities|Casting|CastToCustomGameInstance (Game|GetGameInstance)))
      (Variables|Default|SetSelected%20Expedition%20Expedition%20Type (.expeditiontype (Variables|/Game/DarkMemoireProject/DataManagement/GameData/CustomGameInstance.CustomGameInstance_C|GetSelectedExpedition _ascustom_game_instance)))
      (Variables|Default|SetSelected%20Expedition%20Goal%20Room%20Tag (.goalroomtag (Variables|/Game/DarkMemoireProject/DataManagement/GameData/CustomGameInstance.CustomGameInstance_C|GetSelectedExpedition _ascustom_game_instance)))
      (Variables|Default|SetSelected%20Expedition%20Goal%20Event (.goalevent (Variables|/Game/DarkMemoireProject/DataManagement/GameData/CustomGameInstance.CustomGameInstance_C|GetSelectedExpedition _ascustom_game_instance))))))

(fn ConstructionScript)

(fn SetPlayerStartingLocation
  (bind _roominstances (Variables|Default|GetRoomInstances))
  (bind _room_tags (Variables|Default|GetRoom%20Tags))
  (bind _output (Utilities|Array|Get(acopy) _room_tags))
  (bind _value (Utilities|Map|Find _roominstances _output))
  (Transformation|SetActorLocation (.AsPlayer (Utilities|Casting|CastToPlayer (Game|GetPlayerCharacter 0))) (Transformation|GetActorLocation _value) false true)
  (bind _output_get (Variables|Default|SetCurrentRoom _value))
  (Utilities|Array|Add (Variables|Default|GetRoomsVisited) _output_get))

(fn RemoveRoom
  (params (room :type BP%20Room%20Object%20Reference))
  (Utilities|FlowControl|Sequence
    (:then_0
      (LocalVariables|SetRoomVar room)
      (LocalVariables|SetRoomDoors (Variables|/Game/DarkMemoireProject/Blueprints/Room/BP_Room.BP_Room_C|GetDoors room))
      (LocalVariables|SetRoomObjects (Variables|/Game/DarkMemoireProject/Blueprints/Room/BP_Room.BP_Room_C|GetInteractObjects room))
      (LocalVariables|SetRoomLights (Variables|/Game/DarkMemoireProject/Blueprints/Room/BP_Room.BP_Room_C|GetLightSources room))
      (LocalVariables|SetRoomDarkLights (Variables|/Game/DarkMemoireProject/Blueprints/Room/BP_Room.BP_Room_C|GetDarkLightSources room)))
    (:then_1
      (for _array_element (LocalVariables|GetRoomDoors)
        (Actor|DestroyActor _array_element))
      (for _array_element_2 (LocalVariables|GetRoomObjects)
        (Actor|DestroyActor _array_element_2))
      (for _array_element_3 (LocalVariables|GetRoomLights)
        (Actor|DestroyActor _array_element_3))
      (for _array_element_4 (LocalVariables|GetRoomDarkLights)
        (Actor|DestroyActor _array_element_4))
      (Actor|DestroyActor (LocalVariables|GetRoomVar)))))

(fn RemoveRoomArray
  (params (Rooms :type Array%20of%20BP%20Room%20Object%20References))
  (for _array_element Rooms
    (CallFunction|RemoveRoom _array_element)))

(fn TeleporttoNextDoor
  (params (Door :type BP%20Door%20Object%20Reference))
  (bind _connecteddoor (CallFunction|GetConnectedDoor (Utilities|Array|FindItem (Variables|Default|GetDoorInstances) Door)))
  (Transformation|SetActorLocation (.AsPlayer (Utilities|Casting|CastToPlayer (Game|GetPlayerCharacter 0))) (Transformation|GetWorldLocation (Variables|/Game/DarkMemoireProject/Blueprints/Room/BP_Door.BP_Door_C|GetAreaToLand _connecteddoor)) false false)
  (Pawn|SetControlRotation (Game|GetPlayerController 0) (Math|Rotator|MakeRotator 0.0 0.0 (+ (.Yaw (Math|Rotator|BreakRotator (Math|Rotator|FindLookatRotation (Transformation|GetActorLocation (Game|GetPlayerCharacter 0)) (Transformation|GetActorLocation _connecteddoor)))) 1.8e+02)))
  (bind _room (CallFunction|GetDoorsRoom _connecteddoor))
  (bind _output_get (Variables|Default|SetCurrentRoom _room))
  (return _connecteddoor _output_get))

(fn GetConnectedDoor
  (params (Index :type Integer))
  (bind _connecteddoor (CallFunction|GetConnectedDoorIndex Index))
  (return (Utilities|Array|Get(acopy) (Variables|Default|GetDoorInstances) _connecteddoor)))

(fn GetConnectedDoorIndex
  (params (Index :type Integer))
  (LocalVariables|SetSearchIndex Index)
  (bind _result (Math|Integer|DecrementInt (Utilities|Array|Length (Variables|Default|GetRoomConnections)))
    (:%20%20
      (for _index (range 0 _result)
        (if (!= (LocalVariables|GetSearchIndex) _index)
          (bind _connectionvalue (CallFunction|GetConnection _index (LocalVariables|GetSearchIndex)))
          (if (> _connectionvalue 0)
            (return _index)))))))

(fn GetConnection
  (params (IndexA :type Integer) (IndexB :type Integer))
  (Utilities|FlowControl|Sequence
    (:then_0
      (bind (_newindexx _newindexy) (CallFunction|NormalizeConnectionIndexes IndexA IndexB))
      (LocalVariables|SetIndexX _newindexx)
      (LocalVariables|SetIndexY _newindexy))
    (:then_1
      (return (Utilities|Array|Get(acopy) (Utilities|Struct|BreakST_Array (Utilities|Array|Get(acopy) (Variables|Default|GetRoomConnections) (LocalVariables|GetIndexX))) (LocalVariables|GetIndexY))))))

(fn NormalizeConnectionIndexes
  (params (IndexX :type Integer) (IndexY :type Integer))
  (if (> IndexX IndexY)
    (return IndexX IndexY)
    (else
      (return IndexY IndexX))))

(fn RandomizeDoorsConnections
  (bind (_firstdoor _firstdoorpair _seconddoor _seconddoorpair) (CallFunction|GetDoorPairstoChange))
  (CallFunction|CrossDoorsConnections _firstdoor _firstdoorpair _seconddoor _seconddoorpair)
  (return))

(fn GetDoorPairstoChange
  (bind _doors (LocalVariables|GetDoors))
  (bind _result (Math|Integer|DecrementInt (Utilities|Array|Length (Variables|Default|GetDoorInstances)))
    (:%20%20
      (for _index (range 0 _result)
        (Utilities|Array|Add _doors _index))
      (Utilities|FlowControl|Sequence
        (:then_0
          (Utilities|Array|Shuffle _doors)
          (bind _output_get (LocalVariables|SetDoorA (Utilities|Array|Get(acopy) _doors)))
          (bind _connecteddoor (CallFunction|GetConnectedDoorIndex _output_get))
          (LocalVariables|SetDoorAPair _connecteddoor)
          (bind _output_get_2 (LocalVariables|SetDoorB (Utilities|Array|Get(acopy) _doors 1)))
          (bind _connecteddoor_2 (CallFunction|GetConnectedDoorIndex _output_get_2))
          (LocalVariables|SetDoorBPair _connecteddoor_2))
        (:then_1
          (return (LocalVariables|GetDoorA) (LocalVariables|GetDoorAPair) (LocalVariables|GetDoorB) (LocalVariables|GetDoorBPair)))))))

(fn CrossDoorsConnections
  (params (DoorA :type Integer) (DoorAPair :type Integer) (DoorB :type Integer) (DoorBPair :type Integer))
  (Utilities|FlowControl|Sequence
    (:then_0
      (CallFunction|SetConnectionValue DoorA DoorAPair false)
      (CallFunction|SetConnectionValue DoorB DoorBPair false))
    (:then_1
      (CallFunction|SetConnectionValue DoorA DoorBPair true)
      (CallFunction|SetConnectionValue DoorB DoorAPair true))))

(fn SetConnectionValue
  (params (DoorIn :type Integer) (DoorOut :type Integer) (Connected :type Boolean))
  (bind (_newindexx _newindexy) (CallFunction|NormalizeConnectionIndexes DoorIn DoorOut))
  (Utilities|Array|SetArrayElem (Utilities|Struct|BreakST_Array (Utilities|Array|Get(acopy) (Variables|Default|GetRoomConnections) _newindexx)) _newindexy (Math|Conversions|ToInteger(Boolean) Connected)))

(fn GoBackTown
  (CallFunction|HandleGoBackTown)
  (return))

(fn OnClockUpdate
  (bind _clockturns (Variables|Default|GetClockTurns))
  (Utilities|FlowControl|Sequence
    (:then_0
      ;[1 1 1] Update Dungeon Clock
      (bind _result (Math|Integer|IncrementInt (Variables|Default|GetClockTicks))
        (:%20%20
          (if (>= _result (Variables|Default|GetClockTicksToTurn))
            (Variables|Default|SetClockTicks (- (Variables|Default|GetClockTicks) (Variables|Default|GetClockTicksToTurn)))
            (Math|Integer|IncrementInt (Variables|Default|GetClockTurns)
              (:%20%20
                (Variables|Default|SetClockTurned true)))))))
    (:then_1
      ;[1 1 1] Set Quantity of Events to add
      (if (not (Variables|Default|GetMaxTicksReached))
        (if (>= _clockturns (Variables|Default|GetSecondPhaseTicks))
          (Variables|Default|SetQuantityEvents 3)
          (elif (>= _clockturns (Variables|Default|GetThirdPhaseTicks))
            (Variables|Default|SetQuantityEvents (Utilities|Array|Length (Variables|Default|GetRoom%20Tags)))
            (Variables|Default|SetMaxTicksReached true)))))
    (:then_2
      ;[1 1 1] Update Events on Rooms. If in Third Phase (2 or more clock turns), change room connections. If in third phase (4 or more), reduce sanity on player.
      (if (Variables|Default|GetClockTurned)
        (Variables|Default|SetClockTurned false)
        (CallFunction|AddEventstoRooms (Variables|Default|GetQuantityEvents))
        (if (>= (Variables|Default|GetClockTurns) (Variables|Default|GetThirdPhaseTicks))
          (bind _asplayer (Utilities|Casting|CastToPlayer (Game|GetPlayerCharacter 0)))
          (Variables|/Game/DarkMemoireProject/Blueprints/PlayerCharacter/Player.Player_C|SetCurrentSanity _asplayer (- (Variables|/Game/DarkMemoireProject/Blueprints/PlayerCharacter/Player.Player_C|GetCurrentSanity _asplayer) (- (Variables|Default|GetClockTurns) 3)))
          (CallFunction|RandomizeDoorsConnections :!label _label)
          (elif (>= (Variables|Default|GetClockTurns) (Variables|Default|GetSecondPhaseTicks))
            (goto _label)))))))

(fn AddEventstoRooms
  (params (QuantityEvents :type Integer))
  (bind _emptyrooms (LocalVariables|GetEmptyRooms))
  (bind _eventstoadd (LocalVariables|GetEventsToAdd))
  ;[1 1 1] Generate random events to add to rooms
  (for _index (range 0 (- QuantityEvents 1))
    (bind _event (CallFunction|GenerateEvent (Utilities|String|StringToName (Variables|Default|GetLevelName))))
    (Utilities|Array|Add (LocalVariables|GetEventsToAdd) _event))
  ;[1 1 1] Get rooms without events
  (bind _values (Utilities|Map|Values (Variables|Default|GetRoomInstances)))
  (for _array_element _values
    (if (< (Utilities|Array|Length (Variables|/Game/DarkMemoireProject/Blueprints/Room/BP_Room.BP_Room_C|GetRoomEvent _array_element)) 1)
      (Utilities|Array|Add (LocalVariables|GetEmptyRooms) _array_element)))
  ;[1 1 1] Add an event to a room until there is no room empty or there is no events to add
  (Utilities|Array|Shuffle _emptyrooms)
  (bind _array_element_2 (Utilities|Array|ForEachLoopwithBreak _emptyrooms :!label _label)
    (:LoopBody
      (Utilities|Array|Add (Variables|/Game/DarkMemoireProject/Blueprints/Room/BP_Room.BP_Room_C|GetRoomEvent _array_element_2) (Utilities|Array|Get(acopy) (LocalVariables|GetEventsToAdd)))
      (Utilities|Array|RemoveIndex _eventstoadd)
      (if (== (Utilities|Array|Length _eventstoadd) 0)
        (goto _label Break)))))

(fn AddEventstoInteractiveObjects
  (bind _availableiwos (LocalVariables|GetAvailableIWOs))
  (Utilities|FlowControl|Sequence
    (:then_0
      (bind _outactors (Actor|GetAllActorsOfClass "/Game/DarkMemoireProject/Blueprints/Room/BP_InteractiveObject.BP_InteractiveObject_C"))
      (LocalVariables|SetQuantityIntObjs (/ (* (Utilities|Array|Length _outactors) 2) 3))
      (for _array_element _outactors
        (bind _event_is_ready (Default|IsEventReady _array_element))
        (if (not _event_is_ready)
          (Utilities|Array|Add (LocalVariables|GetAvailableIWOs) _array_element))))
    (:then_1
      (Utilities|Array|Shuffle _availableiwos)
      (bind _array_element_2 (Utilities|Array|ForEachLoopwithBreak _availableiwos :!label _label)
        (:LoopBody
          (bind _event (CallFunction|GenerateEvent (Utilities|String|StringToName (Variables|Default|GetLevelName))))
          (Default|SetEvent _array_element_2 _event)
          (bind _output_get (LocalVariables|SetQuantityIntObjs (- (LocalVariables|GetQuantityIntObjs) 1)))
          (if (not (> _output_get 0))
            (goto _label Break)))))))

(fn RunRoomEvent
  (params (RoomEvent :type ST%20Event%20Structure))
  (CallFunction|RunEvent RoomEvent)
  (return))

(fn GetDoorsRoom
  (params (Door :type BP%20Door%20Object%20Reference))
  (bind _values (Utilities|Map|Values (Variables|Default|GetRoomInstances)))
  (for _array_element _values
    (if (> (Utilities|Array|FindItem (Variables|/Game/DarkMemoireProject/Blueprints/Room/BP_Room.BP_Room_C|GetDoors _array_element) Door) -1)
      (return _array_element)))
  (return 0))

(fn StartCombat
  (params (EnemyData :type ST%20Enemy%20Structure) (EnemyName :type Name))
  (Variables|Default|SetCurrentGameMode 1)
  (Default|TogglePlayerMode (Variables|Default|GetPlayerInstance) true)
  (bind _returnvalue (Game|SpawnActorfromClass "/Game/DarkMemoireProject/Blueprints/Enemy/Enemy.Enemy_C" (Math|Transform|MakeTransform (Transformation|GetActorLocation (Variables|Default|GetCurrentRoom)) "0, 0, 0" "1,1,1") "AlwaysSpawn" 0 EnemyData EnemyName 0))
  (bind _output_get (Variables|Default|SetActiveEnemy _returnvalue))
  (Game|Player|SetViewTargetwithBlend (Game|GetPlayerController 0) _output_get 2.0 "VTBlend_Linear" 0.0 false)
  (Transformation|SetActorRotation (Variables|Default|GetActiveEnemy) (Math|Rotator|FindLookatRotation (Transformation|GetActorLocation (Variables|Default|GetActiveEnemy)) (Transformation|GetActorLocation (Variables|Default|GetPlayerInstance))))
  (Pawn|SetControlRotation (Game|GetPlayerController 0) (Math|Rotator|FindLookatRotation (Transformation|GetActorLocation (Variables|Default|GetPlayerInstance)) (Transformation|GetActorLocation (Variables|Default|GetActiveEnemy)))))

(fn EndCombat
  (Actor|DestroyActor (Variables|Default|GetActiveEnemy))
  (Default|TogglePlayerMode (Variables|Default|GetPlayerInstance) false)
  (Variables|Default|SetCurrentGameMode 0)
  (bind _isalive (Default|IsAlive (Variables|Default|GetPlayerInstance)))
  (if (not _isalive)
    (CallFunction|HandlePlayerDeath)))

(fn ResolveEnemyAction
  (params (ActionData :type ST%20Card%20Structure))
  (CallFunction|ResolveCardAction ActionData (Variables|Default|GetPlayerInstance) (Variables|Default|GetActiveEnemy) "Enemy")
  (return))

(fn ResolvePlayerAction
  (params (ActionData :type ST%20Card%20Structure))
  (CallFunction|ResolveCardAction ActionData (Variables|Default|GetPlayerInstance) (Variables|Default|GetActiveEnemy) "Player")
  (return))

(fn OnGoalAchieved
  (Variables|Default|SetExpeditionAccomplished true)
  (Widget|SetVisibility (Variables|/Game/DarkMemoireProject/UMG/HUD/DungeonHUD.DungeonHUD_C|GetExpeditionAccomplishedMessage (Variables|/Game/DarkMemoireProject/Blueprints/PlayerCharacter/Player.Player_C|GetDungeonHUD (Variables|Default|GetPlayerInstance))) "Visible"))

(fn CheckAllRoomsVisited
  (if (and (== (Utilities|Array|Length (Variables|Default|GetRoom%20Tags)) (Utilities|Array|Length (Variables|Default|GetRoomsVisited))) (Utilities|Enum|Equal(Enum) (Variables|Default|GetSelected%20Expedition%20Expedition%20Type) "NewEnumerator0"))
    (CallFunction|OnGoalAchieved)))