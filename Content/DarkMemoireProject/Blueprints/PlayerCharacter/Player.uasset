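; Player character for dungeon expeditions, loading its job-based mesh and stats (life, stamina, sanity, money) from the save slot.
; Creates the card-deck HUD, relays card clicks through a dispatcher, and toggles between movement and cursor-driven deck modes.
; Handles walking, sprinting and overlap-based interaction with doors and objects, plus a dev shortcut back to town.
; Vertical look rotates a clamped spring arm, leaving the mesh unrotated.
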(event Custom|ToggleMovementRotation
  (params (Move :type Boolean) (Rotate :type Boolean))
  ;[1 1 1] Movement and Camera
  ;;[1 1 1] Toggle CanMove and CanRotate
  (Variables|Default|SetCanMove Move)
  (Variables|Default|SetCanRotate Rotate))

(event Custom|OnCardClicked
  (params (CardIndex :type Integer) (CardData :type ST%20Card%20Structure) (StackedTime :type Integer))
  ;[1 1 1] Initialize HUD
  (Default|CallDispatchCardSelected CardIndex CardData StackedTime))

(event Custom|HandleCardClicked
  (params (CardIndex :type Integer) (CardData :type ST%20Card%20Structure) (StackedTime :type Integer))
  ;[1 1 1] Initialize HUD
  (CallFunction|OnCardClicked CardIndex CardData StackedTime))

(event EventBeginPlay
  (Utilities|FlowControl|Sequence
    (:then_0
      ;[1 1 1] Default character values
      (bind _returnvalue (SaveGame|LoadGamefromSlot "SaveGameSlot"))
      (bind _output_get (Variables|Default|SetSaveGame _returnvalue))
      (bind _assave_game_slot (Utilities|Casting|CastToSaveGameSlot _output_get))
      (CallFunction|SetPlayerMesh (Variables|/Game/DarkMemoireProject/DataManagement/GameData/SaveGameSlot.SaveGameSlot_C|GetJob _assave_game_slot))
      (CallFunction|SetPlayerValues (Variables|/Game/DarkMemoireProject/DataManagement/GameData/SaveGameSlot.SaveGameSlot_C|GetCharacterData _assave_game_slot)))
    (:then_1
      ;[1 1 1] Initialize HUD
      (bind _ascustom_game_instance (Utilities|Casting|CastToCustomGameInstance (Game|GetGameInstance)))
      (bind _returnvalue_2 (UserInterface|CreateWidget "/Game/DarkMemoireProject/UMG/HUD/DungeonHUD.DungeonHUD_C" 0 (Variables|/Game/DarkMemoireProject/DataManagement/GameData/CustomGameInstance.CustomGameInstance_C|GetCards _ascustom_game_instance)))
      (bind _output_get_2 (Variables|Default|SetDungeonHUD _returnvalue_2))
      (EventDispatchers|BindEventtoDispatchCardClicked _output_get_2 (delegate Custom|HandleCardClicked))
      (UserInterface|Viewport|AddtoViewport _output_get_2 0)
      (Input|SetInputModeGameOnly (Game|GetPlayerController 0))
      (CallFunction|TogglePlayerMode false))))

(event Collision|EventActorBeginOverlap
  (params (OtherActor :type Actor%20Object%20Reference))
  ;[1 1 1] Manage interaction with objects/doors in game. Also quit option for fast dev.
  ;;[1 1 1] Save object we are overlapping with to check later what to do if press E
  (Variables|Default|SetObjectOnReach OtherActor))

(event Collision|EventActorEndOverlap
  (params (OtherActor :type Actor%20Object%20Reference))
  ;[1 1 1] Manage interaction with objects/doors in game. Also quit option for fast dev.
  ;;[1 1 1] Save object we are overlapping with to check later what to do if press E
  (if (== OtherActor (Variables|Default|GetObjectOnReach))
    (Variables|Default|SetObjectOnReach 0)))

(event Input|ActionEvents|InputActionActionKeys
  (params (Key :type Key%20Structure :default "None"))
  ;[1 1 1] Manage interaction with objects/doors in game. Also quit option for fast dev.
  (:Pressed
    (if (== Key "Q")
      (bind _asdungeon_mode (Utilities|Casting|CastToDungeonMode (Game|GetGameMode)))
      (Default|GoBackTown _asdungeon_mode)
      (elif (== Key "E")
        ;;[1 1 1] Interaction with door runs function
        (bind _asbp_door (Utilities|Casting|CastToBP_Door (Variables|Default|GetObjectOnReach))
          (:then
            (Default|OnOpenDoor _asbp_door))
          (:CastFailed
            ;;[1 1 1] Interaction with object runs function
            (bind _asbp_interactive_object (Utilities|Casting|CastToBP_InteractiveObject (Variables|Default|GetObjectOnReach)))
            (Default|OnObjectActivated _asbp_interactive_object)))))))

(event Input|AxisEvents|InputAxisMoveForwardBackward
  (params (AxisValue :type Float%20%28single-precision%29))
  ;[1 1 1] Movement and Camera
  ;;[1 1 1] Forward/Backward Movement with Sprint
  (if (Variables|Default|GetCanMove)
    (Pawn|Input|AddMovementInput (Transformation|GetActorForwardVector) AxisValue false)
    (if (not (>= AxisValue 0.0))
      (Variables|/Script/Engine.CharacterMovementComponent|SetMaxWalkSpeed (Variables|Character|GetCharacterMovement) 2.5e+02))))

(event Input|AxisEvents|InputAxisMoveRightLeft
  (params (AxisValue :type Float%20%28single-precision%29))
  ;[1 1 1] Movement and Camera
  ;;[1 1 1] Lateral Movement
  (if (Variables|Default|GetCanMove)
    (Pawn|Input|AddMovementInput (Transformation|GetActorRightVector) AxisValue false)))

(event Input|AxisEvents|InputAxisLookAtUpDown
  (params (AxisValue :type Float%20%28single-precision%29))
  ;[1 1 1] Movement and Camera
  ;;[1 1 1] Look At Up and Down. Based on Spring Arm to manage weird angles and LookAt without changing mesh rotation.
  (if (Variables|Default|GetCanRotate)
    (Transformation|AddLocalRotation (Variables|Default|GetSpringArm) (Math|Rotator|MakeRotator 0.0 AxisValue 0.0) false false)
    (Transformation|SetRelativeRotation (Variables|Default|GetSpringArm) (Math|Rotator|MakeRotator 0.0 (Math|Float|ClampAngle (.Pitch (Math|Rotator|BreakRotator (Class|SpringArmComponent|GetTargetRotation (Variables|Default|GetSpringArm)))) -45.0 6e+01) 0.0) false false)))

(event Input|AxisEvents|InputAxisLookAtRightLeft
  (params (AxisValue :type Float%20%28single-precision%29))
  ;[1 1 1] Movement and Camera
  ;;[1 1 1] Lateral LookAt
  (if (Variables|Default|GetCanRotate)
    (Pawn|Input|AddControllerYawInput AxisValue)))

(event Input|KeyboardEvents|LeftShift
  (params (Key :type Key%20Structure :default "None"))
  (bind _charactermovement (Variables|Character|GetCharacterMovement))
  ;[1 1 1] Movement and Camera
  ;;[1 1 1] Forward/Backward Movement with Sprint
  ;;;[1 1 1] SPRINT
  (:Pressed
    (if (>= (stale Input|AxisEvents|InputAxisMoveForwardBackward AxisValue) 0.0)
      (Variables|/Script/Engine.CharacterMovementComponent|SetMaxWalkSpeed _charactermovement 5e+02)
      (else
        (Variables|/Script/Engine.CharacterMovementComponent|SetMaxWalkSpeed _charactermovement 2.5e+02 :!label _label))))
  (:Released
    (goto _label)))

(fn ConstructionScript)

(fn SetPlayerMesh
  (params (Job :type String))
  (bind _mesh (Variables|Character|GetMesh))
  (switch string Job
    (:Heir
      ;[1 1 1] Heir Mesh
      (Class|SkinnedMeshComponent|SetSkeletalMesh _mesh "/Game/DarkMemoireProject/Assets/Heir/Maria_J_J_Ong.Maria_J_J_Ong" true)
      (Transformation|SetRelativeScale3D _mesh "1.000000,1.000000,1.000000")
      (Class|SkeletalMeshComponent|SetAnimClass _mesh "/Game/DarkMemoireProject/Animations/Heir/Heir_AnimBP.Heir_AnimBP_C"))
    (:Detective
      ;[1 1 1] Detective Mesh
      (Class|SkinnedMeshComponent|SetSkeletalMesh _mesh "/Game/DarkMemoireProject/Assets/Detective/Eve_By_J_Gonzales.Eve_By_J_Gonzales" true)
      (Transformation|SetRelativeScale3D _mesh (* (Variables|/Script/Engine.SceneComponent|GetRelativeScale3D _mesh) 1.25))
      (Class|SkeletalMeshComponent|SetAnimClass _mesh "/Game/DarkMemoireProject/Animations/Detective/Detective_AnimBP.Detective_AnimBP_C"))))

(fn SetPlayerValues
  (params (CharacterData :type ST%20Character%20Structure))
  (bind (_life _stamina _sanity _light _basedamage _baseresistance _basespeed _baseaccuracy _basecritical _basecards _description _icon _deployed _chartemplatetype _money) (Utilities|Struct|BreakST_Character CharacterData))
  (bind _output_get (Variables|Default|SetMaxLife _life))
  (Variables|Default|SetCurrentLife _output_get)
  (bind _output_get_2 (Variables|Default|SetMaxStamina _stamina))
  (Variables|Default|SetCurrentStamina _output_get_2)
  (bind _output_get_3 (Variables|Default|SetMaxSanity _sanity))
  (Variables|Default|SetCurrentSanity _output_get_3)
  (Variables|Default|SetLight _light)
  (Variables|Default|SetBase%20Damage _basedamage)
  (Variables|Default|SetBase%20Resistance _baseresistance)
  (Variables|Default|SetBase%20Speed _basespeed)
  (Variables|Default|SetBase%20Accuracy _baseaccuracy)
  (Variables|Default|SetBase%20Critical _basecritical)
  (Variables|Default|SetIcon _icon)
  (bind _output_get_4 (Variables|Default|SetCurrentMoney _money))
  (Variables|Default|SetExpeditionMoney _output_get_4))

(fn GetSanityRatio
  (return (/ (Math|Conversions|ToFloat(Integer) (Variables|Default|GetCurrentSanity)) (Math|Conversions|ToFloat(Integer) (Variables|Default|GetMaxSanity)))))

(fn TogglePlayerMode
  (params (UIMode :type Boolean))
  (bind _returnvalue (not UIMode))
  (CallFunction|ToggleMovementRotation _returnvalue _returnvalue)
  (bind _output_get (Variables|/Script/Engine.PlayerController|SetbShowMouseCursor (Game|GetPlayerController 0) UIMode))
  (if _output_get
    (Default|ShowDeck (Variables|Default|GetDungeonHUD))
    (else
      (Default|HideDeck (Variables|Default|GetDungeonHUD)))))

(fn IsAlive
  (return (and (> (Variables|Default|GetCurrentLife) 0) (> (Variables|Default|GetCurrentSanity) 0))))

(fn ReceiveDamage
  (params (Damage :type Integer))
  (Variables|Default|SetCurrentLife (- (Variables|Default|GetCurrentLife) Damage))
  (return))

(fn ReceiveSanityDamage
  (params (SanityDamage :type Integer))
  (Variables|Default|SetCurrentSanity (- (Variables|Default|GetCurrentSanity) SanityDamage))
  (return))