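; WillOWisp is an enemy Blueprint for a will-o'-wisp that visibly shrinks once it is badly hurt.
; It caches its starting life from EnemyData on BeginPlay.
; ReceiveDamage calls the parent's damage logic, then, the first time life is at or below half, sets a ReducedFire flag and shrinks the Wisp component along its local X axis.
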(event EventBeginPlay
  (|CallParentFunction)
  (Variables|Default|SetBaseLife (.life (Variables|Default|GetEnemyData))))

(event Collision|EventActorBeginOverlap
  (params (OtherActor :type Actor%20Object%20Reference)))

(event EventTick
  (params (DeltaSeconds :type Float%20%28single-precision%29)))

(fn ConstructionScript
  (|CallParentFunction))

(fn ReceiveDamage
  (params (Damage :type Integer))
  (|CallParentFunction Damage)
  (if (and (<= (.life (Variables|Default|GetEnemyData)) (/ (Variables|Default|GetBaseLife) 2)) (not (Variables|Default|GetReducedFire)))
    (Variables|Default|SetReducedFire true)
    (Transformation|SetRelativeScale3D (Variables|Default|GetWisp) "0.300000,1.000000,1.000000")))