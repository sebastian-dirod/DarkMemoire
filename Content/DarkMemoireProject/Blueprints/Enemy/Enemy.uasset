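; Enemy actor for the dungeon game, with data-driven stats and a placeholder idle animation.
; On BeginPlay it fills its Stats struct from the hardcoded TestEnemy row of the DB_Enemies data table.
; A timeline fakes the idle by bobbing the static mesh vertically, playing forward then reversing, with a short random delay before each new cycle.
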(event Custom|FakeIdle_1
  (bind (_direction _newtrack_0) (Timeline|Timeline_0 Play)
    (:Update
      (Transformation|SetRelativeLocation (Variables|Default|GetStaticMesh) (Math|Vector|Lerp(Vector) "0, 0, 0" "0, 0,-20.000000" _newtrack_0) false false))
    (:Finished
      (switch Utilities|FlowControl|Switch|SwitchonETimelineDirection _direction
        (:Forward
          (CallFunction|FakeIdle2))
        (:Backward
          (Utilities|FlowControl|Delay (Math|Random|RandomFloatinRange 0.01 0.25))
          (CallFunction|FakeIdle1))))))

(event Custom|FakeIdle_2
  (bind (_direction _newtrack_0) (Timeline|Timeline_0 Reverse)
    (:Update
      (Transformation|SetRelativeLocation (Variables|Default|GetStaticMesh) (Math|Vector|Lerp(Vector) "0, 0, 0" "0, 0,-20.000000" _newtrack_0) false false))
    (:Finished
      (switch Utilities|FlowControl|Switch|SwitchonETimelineDirection _direction
        (:Forward
          (CallFunction|FakeIdle2))
        (:Backward
          (Utilities|FlowControl|Delay (Math|Random|RandomFloatinRange 0.01 0.25))
          (CallFunction|FakeIdle1))))))

(event EventBeginPlay
  (CallFunction|FakeIdle1)
  (bind _returnvalue (Utilities|GetDataTableRow "/Game/DarkMemoireProject/DataManagement/Tables/DB_Enemies.DB_Enemies" "TestEnemy")
    (:then
      (Utilities|Struct|SetmembersinST_Enemy (Variables|Default|GetStats) (.Life (Utilities|Struct|BreakST_Enemy _returnvalue)) (.Stamina (Utilities|Struct|BreakST_Enemy _returnvalue)) (.BaseDamage (Utilities|Struct|BreakST_Enemy _returnvalue)) (.BaseResistance (Utilities|Struct|BreakST_Enemy _returnvalue)) (.BaseSpeed (Utilities|Struct|BreakST_Enemy _returnvalue)) (.BaseAccuracy (Utilities|Struct|BreakST_Enemy _returnvalue)) (.BaseCritical (Utilities|Struct|BreakST_Enemy _returnvalue)) (.ActionCards (Utilities|Struct|BreakST_Enemy _returnvalue)) (.Description (Utilities|Struct|BreakST_Enemy _returnvalue)) (.Icon (Utilities|Struct|BreakST_Enemy _returnvalue)) (.EnemyActor (Utilities|Struct|BreakST_Enemy _returnvalue)) (.DungeonID (Utilities|Struct|BreakST_Enemy _returnvalue))))))

(fn ConstructionScript)