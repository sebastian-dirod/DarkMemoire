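; Function library that generates and runs random dungeon events: Combat, Fortune, Peril or Lore.
; GenerateEvent picks a type at random and builds an STEvent, filtering DB_Enemies by dungeon ID and DB_LoreEntries by current level name.
; RunEvent dispatches that struct to start combat through DungeonMode, grant an item or money, worsen a player stat, or display lore.
; Non-combat outcomes show their messages on the player's DungeonHUD.
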(fn GenerateEvent
  (params (DungeonID :type Name))
  (switch int (Math|Random|RandomIntegerinRange 0 3)
    (:0
      (bind _event (CallFunction|GenerateCombat DungeonID))
      (return _event))
    (:1
      (bind _event_2 (CallFunction|GenerateFortune))
      (return _event_2))
    (:2
      (bind _event_3 (CallFunction|GeneratePeril))
      (return _event_3))
    (:3
      (bind _event_4 (CallFunction|GenerateLore))
      (return _event_4))))

(fn GenerateCombat
  (params (DungeonID :type Name))
  (bind _enemynames (LocalVariables|GetEnemyNames))
  (LocalVariables|SetDungeonName DungeonID)
  (bind _outrownames (DataTable|GetDataTableRowNames "/Game/DarkMemoireProject/DataManagement/Tables/DB_Enemies.DB_Enemies"))
  (for _array_element _outrownames
    (bind _returnvalue (Utilities|GetDataTableRow "/Game/DarkMemoireProject/DataManagement/Tables/DB_Enemies.DB_Enemies" _array_element)
      (:then
        (if (Utilities|Name|Equal(Name) (.DungeonID (Utilities|Struct|BreakST_Enemy _returnvalue)) (LocalVariables|GetDungeonName))
          (Utilities|Map|Add (LocalVariables|GetEnemyNames) _array_element _returnvalue)))))
  (bind _keys (Utilities|Map|Keys _enemynames))
  (return (Utilities|Struct|MakeST_Event "NewEnumerator0" "" "None" (Utilities|Array|Get(acopy) _keys (Math|Random|RandomInteger (Utilities|Array|Length _keys))) (.Value (Utilities|Map|Find _enemynames (Utilities|Array|Get(acopy) _keys (Math|Random|RandomInteger (Utilities|Array|Length _keys))))) "None" true)))

(fn GenerateFortune
  (return (Utilities|Struct|MakeST_Event "NewEnumerator1" "" "None" "None" "(Life_32_769D51C34EBE63AC1FF18B9C5A759C0C=0,Stamina_20_A28EABF845C0BECAC361C3951BB2D0BB=100,BaseDamage_22_F50C29B84DD4993BFE61A18C6684B75E=0,BaseResistance_29_A3B080F84032DE4224BE0EA182EE74EA=0,BaseSpeed_24_BDEFE8804EC1373059381080797DC1AF=0,BaseAccuracy_45_AC4677114C09A1640686C68C763DBDCE=0.000000,BaseCritical_26_A023684A48D1B749EFA428826A4CD630=0.000000,ActionCards_63_D6C094064595230D39F1C7963D44CEC5=(),Description_44_1BF8FE1D46A2ECC80AF504884503FF9D=,Icon_48_413DEB9A4E72FAF92DFD0CA214537B82=None,EnemyActor_68_0A23F5244E19B51A719D26A25D739504=None,DungeonID_71_AE961B9D44BFDF233A299D82C9E45B91=\"ShunnedHouse\")" "None" true)))

(fn GeneratePeril
  (return (Utilities|Struct|MakeST_Event "NewEnumerator2" (.OutItem (Utilities|Array|Random (Utilities|Array|MakeArray "Damage" "Resistance" "Speed" "Money" "Sanity"))) "None" "None" "(Life_32_769D51C34EBE63AC1FF18B9C5A759C0C=0,Stamina_20_A28EABF845C0BECAC361C3951BB2D0BB=100,BaseDamage_22_F50C29B84DD4993BFE61A18C6684B75E=0,BaseResistance_29_A3B080F84032DE4224BE0EA182EE74EA=0,BaseSpeed_24_BDEFE8804EC1373059381080797DC1AF=0,BaseAccuracy_45_AC4677114C09A1640686C68C763DBDCE=0.000000,BaseCritical_26_A023684A48D1B749EFA428826A4CD630=0.000000,ActionCards_63_D6C094064595230D39F1C7963D44CEC5=(),Description_44_1BF8FE1D46A2ECC80AF504884503FF9D=,Icon_48_413DEB9A4E72FAF92DFD0CA214537B82=None,EnemyActor_68_0A23F5244E19B51A719D26A25D739504=None,DungeonID_71_AE961B9D44BFDF233A299D82C9E45B91=\"ShunnedHouse\")" "None" true)))

(fn GenerateLore
  (bind _outrownames (DataTable|GetDataTableRowNames "/Game/DarkMemoireProject/DataManagement/Tables/DB_LoreEntries.DB_LoreEntries"))
  (bind _returnvalue (Game|GetCurrentLevelName 0))
  (LocalVariables|SetLevelName _returnvalue)
  (for _array_element _outrownames
    (bind _returnvalue_2 (Utilities|GetDataTableRow "/Game/DarkMemoireProject/DataManagement/Tables/DB_LoreEntries.DB_LoreEntries" _array_element)
      (:then
        (if (Utilities|Name|Equal(Name) (.DungeonID (Utilities|Struct|BreakST_LoreEntry _returnvalue_2)) (Utilities|String|StringToName (LocalVariables|GetLevelName)))
          (Utilities|Array|Add (LocalVariables|GetDungeonLoreEntries) _array_element)))))
  (return (Utilities|Struct|MakeST_Event "NewEnumerator3" "" "None" "None" "(Life_32_769D51C34EBE63AC1FF18B9C5A759C0C=0,Stamina_20_A28EABF845C0BECAC361C3951BB2D0BB=100,BaseDamage_22_F50C29B84DD4993BFE61A18C6684B75E=0,BaseResistance_29_A3B080F84032DE4224BE0EA182EE74EA=0,BaseSpeed_24_BDEFE8804EC1373059381080797DC1AF=0,BaseAccuracy_45_AC4677114C09A1640686C68C763DBDCE=0.000000,BaseCritical_26_A023684A48D1B749EFA428826A4CD630=0.000000,ActionCards_63_D6C094064595230D39F1C7963D44CEC5=(),Description_44_1BF8FE1D46A2ECC80AF504884503FF9D=,Icon_48_413DEB9A4E72FAF92DFD0CA214537B82=None,EnemyActor_68_0A23F5244E19B51A719D26A25D739504=None,DungeonID_71_AE961B9D44BFDF233A299D82C9E45B91=\"ShunnedHouse\")" (.OutItem (Utilities|Array|Random (LocalVariables|GetDungeonLoreEntries))) true)))

(fn RunEvent
  (params (EventData :type ST%20Event%20Structure))
  (bind (_eventtype _statistic _item _enemy _enemydata _lore) (Utilities|Struct|BreakST_Event EventData))
  (bind _output_get (LocalVariables|SetEventType _eventtype))
  (LocalVariables|SetStatisticName _statistic)
  (LocalVariables|SetItemName _item)
  (LocalVariables|SetEnemyName _enemy)
  (LocalVariables|SetEnemyData _enemydata)
  (LocalVariables|SetLoreEntryName _lore)
  (switch Utilities|FlowControl|Switch|SwitchonEEventType _output_get
    (:NewEnumerator0
      (CallFunction|RunCombat (LocalVariables|GetEnemyData) (LocalVariables|GetEnemyName)))
    (:NewEnumerator1
      (CallFunction|RunFortune (LocalVariables|GetItemName)))
    (:NewEnumerator2
      (CallFunction|RunPeril (Utilities|String|StringToName (LocalVariables|GetStatisticName))))
    (:NewEnumerator3
      (CallFunction|RunLore (LocalVariables|GetLoreEntryName))))
  (return))

(fn RunCombat
  (params (EnemyData :type ST%20Enemy%20Structure) (EnemyName :type Name))
  (LocalVariables|SetData EnemyData)
  (LocalVariables|SetName EnemyName)
  (bind _asdungeon_mode (Utilities|Casting|CastToDungeonMode (Game|GetGameMode)))
  (Default|StartCombat _asdungeon_mode (LocalVariables|GetData) (LocalVariables|GetName))
  (return))

(fn RunFortune
  (params (ItemName :type Name))
  (bind _asplayer (Utilities|Casting|CastToPlayer (Game|GetPlayerCharacter 0)))
  (bind _output_get (LocalVariables|SetPlayer _asplayer))
  (LocalVariables|SetHUD (Variables|/Game/DarkMemoireProject/Blueprints/PlayerCharacter/Player.Player_C|GetDungeonHUD _output_get))
  (if (Utilities|Name|NotEqual(Name) ItemName "None")
    (Utilities|Array|Add (Variables|/Game/DarkMemoireProject/Blueprints/PlayerCharacter/Player.Player_C|GetAcquiredItems (LocalVariables|GetPlayer)) ItemName)
    (Default|ShowMessage (LocalVariables|GetHUD) (Utilities|String|Append "You have found " (Utilities|String|ToString(Name) ItemName) " !"))
    (else
      (bind _output_get_2 (LocalVariables|SetMoneyFound (Math|Random|RandomIntegerinRange 25 75)))
      (Variables|/Game/DarkMemoireProject/Blueprints/PlayerCharacter/Player.Player_C|SetExpeditionMoney (LocalVariables|GetPlayer) (+ (Variables|/Game/DarkMemoireProject/Blueprints/PlayerCharacter/Player.Player_C|GetExpeditionMoney (LocalVariables|GetPlayer)) _output_get_2))
      (Default|ShowMessage (LocalVariables|GetHUD) (Utilities|String|Append "You have found " (Utilities|String|ToString(Integer) _output_get_2) " pounds!")))))

(fn RunPeril
  (params (Statistic :type Name))
  (bind _asplayer (Utilities|Casting|CastToPlayer (Game|GetPlayerCharacter 0)))
  (bind _output_get (LocalVariables|SetPlayer _asplayer))
  (LocalVariables|SetHUD (Variables|/Game/DarkMemoireProject/Blueprints/PlayerCharacter/Player.Player_C|GetDungeonHUD _output_get))
  (switch name Statistic
    (:Damage
      (Math|Integer|DecrementInt (Variables|/Game/DarkMemoireProject/Blueprints/PlayerCharacter/Player.Player_C|GetBase%20Damage (LocalVariables|GetPlayer))
        (:%20%20
          (Default|ShowMessage (LocalVariables|GetHUD) "Oh, the fear... how it attacks the nerves and makes you less effective."))))
    (:Resistance
      (Math|Integer|DecrementInt (Variables|/Game/DarkMemoireProject/Blueprints/PlayerCharacter/Player.Player_C|GetBase%20Resistance (LocalVariables|GetPlayer))
        (:%20%20
          (Default|ShowMessage (LocalVariables|GetHUD) "The air weights in your lungs... as if it was the start of an illness. You feel less resistant than before"))))
    (:Speed
      (Math|Integer|IncrementInt (Variables|/Game/DarkMemoireProject/Blueprints/PlayerCharacter/Player.Player_C|GetBase%20Speed (LocalVariables|GetPlayer))
        (:%20%20
          (Default|ShowMessage (LocalVariables|GetHUD) "The coldness of the place gets you numb and tired. You feel slower than before..."))))
    (:Money
      (Variables|/Game/DarkMemoireProject/Blueprints/PlayerCharacter/Player.Player_C|SetExpeditionMoney (LocalVariables|GetPlayer) (- (Variables|/Game/DarkMemoireProject/Blueprints/PlayerCharacter/Player.Player_C|GetExpeditionMoney (LocalVariables|GetPlayer)) 10))
      (Default|ShowMessage (LocalVariables|GetHUD) "You have lost some money!"))
    (:Sanity
      (Variables|/Game/DarkMemoireProject/Blueprints/PlayerCharacter/Player.Player_C|SetCurrentSanity (LocalVariables|GetPlayer) (- (Variables|/Game/DarkMemoireProject/Blueprints/PlayerCharacter/Player.Player_C|GetCurrentSanity (LocalVariables|GetPlayer)) 5))
      (Default|ShowMessage (LocalVariables|GetHUD) "You felt a weird presence and lost partial sanity"))))

(fn RunLore
  (params (EntryName :type Name))
  (bind _asplayer (Utilities|Casting|CastToPlayer (Game|GetPlayerCharacter 0)))
  (bind _returnvalue (Utilities|GetDataTableRow "/Game/DarkMemoireProject/DataManagement/Tables/DB_LoreEntries.DB_LoreEntries" EntryName)
    (:then
      (Default|ShowMessage (Variables|/Game/DarkMemoireProject/Blueprints/PlayerCharacter/Player.Player_C|GetDungeonHUD _asplayer) (Utilities|String|Append "You found some notes: " (.LoreText (Utilities|Struct|BreakST_LoreEntry _returnvalue)))))))