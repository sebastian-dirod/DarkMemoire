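; Card combat function library that resolves a played Punch or Shoot card between the player and an enemy.
; ResolveCardAction deducts stamina and sanity for player actions, then dispatches on card ID.
; Each card randomizes damage around the source's base damage, subtracts target resistance and calls ReceiveDamage.
; Shoot can crit for double a fresh roll, using the player's crit stat or a fixed enemy chance.
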(fn ResolveCardAction
  (params (ActionData :type ST%20Card%20Structure) (Player :type Player%20Object%20Reference) (Enemy :type Enemy%20Object%20Reference) (SourceID :type Name))
  (LocalVariables|SetPlayerActor Player)
  (LocalVariables|SetEnemyActor Enemy)
  (LocalVariables|SetSourceActorID SourceID)
  (bind _output_get (LocalVariables|SetSelectedAction ActionData))
  (if (Utilities|Name|Equal(Name) (LocalVariables|GetSourceActorID) "Player")
    (CallFunction|ResolvePlayerActionCosts (.consumedenergy (.carddata _output_get)) (.consumedsanity (.carddata _output_get))))
  (switch name (.cardid (.carddata _output_get))
    (:Punch
      (CallFunction|Punch (LocalVariables|GetPlayerActor) (LocalVariables|GetEnemyActor) (LocalVariables|GetSourceActorID)))
    (:Shoot
      (CallFunction|Shoot (LocalVariables|GetPlayerActor) (LocalVariables|GetEnemyActor) (LocalVariables|GetSourceActorID))))
  (return))

(fn Punch
  (params (Player :type Player%20Object%20Reference) (Enemy :type Enemy%20Object%20Reference) (SourceID :type Name))
  (LocalVariables|SetPlayerActor Player)
  (LocalVariables|SetEnemyActor Enemy)
  (Development|PrintString 0 (Utilities|String|ToString(Name) SourceID) true true "(R=1.000000,G=0.009094,B=0.000000,A=1.000000)" 5.0)
  (switch name SourceID
    (:Player
      (bind _damage (CallFunction|GetPlayerDamage))
      (bind _resistance (CallFunction|GetEnemyResistance (LocalVariables|GetEnemyActor)))
      (Default|ReceiveDamage (LocalVariables|GetEnemyActor) (- (Math|Random|RandomIntegerinRange (Math|Float|Truncate (* _damage 0.8)) (Math|Float|Truncate (* _damage 1.2))) _resistance)))
    (:Enemy
      (bind _damage_2 (CallFunction|GetEnemyDamage (LocalVariables|GetEnemyActor)))
      (Development|PrintString 0 (Utilities|String|ToString(Integer) (Math|Random|RandomIntegerinRange (Math|Float|Truncate (* _damage_2 0.7)) (Math|Float|Truncate (* _damage_2 1.3)))) true true "(R=0.479167,G=0.397418,B=0.000000,A=1.000000)" 5.0)
      (bind _resistance_2 (CallFunction|GetPlayerResistance))
      (Development|PrintString 0 (Utilities|String|ToString(Integer) (- (Math|Random|RandomIntegerinRange (Math|Float|Truncate (* _damage_2 0.7)) (Math|Float|Truncate (* _damage_2 1.3))) _resistance_2)) true true "(R=0.000000,G=0.660000,B=1.000000,A=1.000000)" 5.0)
      (Default|ReceiveDamage (LocalVariables|GetPlayerActor) (- (Math|Random|RandomIntegerinRange (Math|Float|Truncate (* _damage_2 0.7)) (Math|Float|Truncate (* _damage_2 1.3))) _resistance_2))))
  (return))

(fn Shoot
  (params (Player :type Player%20Object%20Reference) (Enemy :type Enemy%20Object%20Reference) (SourceID :type Name))
  (LocalVariables|SetPlayerActor Player)
  (LocalVariables|SetEnemyActor Enemy)
  (Development|PrintString 0 (Utilities|String|ToString(Name) SourceID) true true "(R=1.000000,G=0.009094,B=0.000000,A=1.000000)" 5.0)
  (switch name SourceID
    (:Player
      (bind _damage (CallFunction|GetPlayerDamage))
      (LocalVariables|SetDamageDone (Math|Random|RandomIntegerinRange (Math|Float|Truncate (* _damage 0.7)) (Math|Float|Truncate (* _damage 1.3))))
      (bind _criticalchance (CallFunction|GetPlayerCriticalChance))
      (if (>= _criticalchance (Math|Random|RandomFloat))
        (LocalVariables|SetDamageDone (* (Math|Random|RandomIntegerinRange (Math|Float|Truncate (* _damage 0.7)) (Math|Float|Truncate (* _damage 1.3))) 2)))
      (bind _resistance (CallFunction|GetEnemyResistance (LocalVariables|GetEnemyActor)))
      (Default|ReceiveDamage (LocalVariables|GetEnemyActor) (- (LocalVariables|GetDamageDone) _resistance)))
    (:Enemy
      (bind _damage_2 (CallFunction|GetEnemyDamage (LocalVariables|GetEnemyActor)))
      (LocalVariables|SetDamageDone (Math|Random|RandomIntegerinRange (Math|Float|Truncate (* _damage_2 0.6)) (Math|Float|Truncate (* _damage_2 1.4))))
      (if (>= 0.35 (Math|Random|RandomFloat))
        (bind _output_get (LocalVariables|SetDamageDone (* (Math|Random|RandomIntegerinRange (Math|Float|Truncate (* _damage_2 0.6)) (Math|Float|Truncate (* _damage_2 1.4))) 2)))
        (Development|PrintString 0 (Utilities|String|ToString(Integer) _output_get) true true "(R=0.479167,G=0.397418,B=0.000000,A=1.000000)" 5.0))
      (bind _resistance_2 (CallFunction|GetPlayerResistance))
      (Development|PrintString 0 (Utilities|String|ToString(Integer) (- (LocalVariables|GetDamageDone) _resistance_2)) true true "(R=0.000000,G=0.660000,B=1.000000,A=1.000000)" 5.0)
      (Default|ReceiveDamage (LocalVariables|GetPlayerActor) (- (LocalVariables|GetDamageDone) _resistance_2))))
  (return))

(fn ResolvePlayerActionCosts
  (params (Energy :type Integer) (Sanity :type Integer))
  (bind _asplayer (Utilities|Casting|CastToPlayer (Game|GetPlayerCharacter 0)))
  (Variables|/Game/DarkMemoireProject/Blueprints/PlayerCharacter/Player.Player_C|SetCurrentSanity _asplayer (- (Variables|/Game/DarkMemoireProject/Blueprints/PlayerCharacter/Player.Player_C|GetCurrentSanity _asplayer) Sanity))
  (Variables|/Game/DarkMemoireProject/Blueprints/PlayerCharacter/Player.Player_C|SetCurrentStamina _asplayer (- (Variables|/Game/DarkMemoireProject/Blueprints/PlayerCharacter/Player.Player_C|GetCurrentStamina _asplayer) Energy))
  (return))

(fn GetPlayerDamage
  (bind _asplayer (Utilities|Casting|CastToPlayer (Game|GetPlayerCharacter 0)))
  (return (Variables|/Game/DarkMemoireProject/Blueprints/PlayerCharacter/Player.Player_C|GetBase%20Damage _asplayer)))

(fn GetEnemyDamage
  (params (Enemy :type Enemy%20Object%20Reference))
  (return (.basedamage (Variables|/Game/DarkMemoireProject/Blueprints/Enemy/Enemy.Enemy_C|GetEnemyData Enemy))))

(fn GetPlayerResistance
  (bind _asplayer (Utilities|Casting|CastToPlayer (Game|GetPlayerCharacter 0)))
  (return (Variables|/Game/DarkMemoireProject/Blueprints/PlayerCharacter/Player.Player_C|GetBase%20Resistance _asplayer)))

(fn GetEnemyResistance
  (params (Enemy :type Enemy%20Object%20Reference))
  (return (.baseresistance (Variables|/Game/DarkMemoireProject/Blueprints/Enemy/Enemy.Enemy_C|GetEnemyData Enemy))))

(fn GetPlayerCriticalChance
  (bind _asplayer (Utilities|Casting|CastToPlayer (Game|GetPlayerCharacter 0)))
  (return (Variables|/Game/DarkMemoireProject/Blueprints/PlayerCharacter/Player.Player_C|GetBase%20Critical _asplayer)))