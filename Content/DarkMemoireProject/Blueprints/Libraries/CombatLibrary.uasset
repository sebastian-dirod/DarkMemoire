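; Blueprint library that resolves one turn of card combat between the player and an enemy.
; LaunchCard draws a random enemy card from DB_Cards; the lower ConsumedTime plus BaseSpeed strikes first, with ties favoring the player.
; CardAction exchanges BaseDamage hits, writing stats back to the Player and stopping on death.
; If both survive, CardType decrements limited usages and removes spent cards from the GameInstance; death handlers and CardFate are stubs.
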(fn LaunchCard
  (params (Card :type ST%20Card%20Structure))
  (bind _returnvalue (Game|GetPlayerCharacter 0))
  (bind _asplayer (Utilities|Casting|CastToPlayer _returnvalue))
  (LocalVariables|SetPlayerLaunchedCard Card)
  (LocalVariables|SetCharacterData (Variables|/Game/DarkMemoireProject/Blueprints/PlayerCharacter/Player.Player_C|GetCharacter%20Data _asplayer))
  (LocalVariables|SetEnemyData (Variables|/Game/DarkMemoireProject/Blueprints/PlayerCharacter/Player.Player_C|GetEnemyData _asplayer))
  (bind _keys (Utilities|Map|Keys (.ActionCards (Utilities|Struct|BreakST_Enemy (Variables|/Game/DarkMemoireProject/Blueprints/PlayerCharacter/Player.Player_C|GetEnemyData _asplayer)))))
  (bind _returnvalue_2 (Utilities|GetDataTableRow "/Game/DarkMemoireProject/DataManagement/Tables/DB_Cards.DB_Cards" (.OutItem (Utilities|Array|Random _keys)))
    (:then
      (LocalVariables|SetEnemyLaunchedCard _returnvalue_2)
      (Development|PrintString 0)
      (if (<= (+ (.ConsumedTime (Utilities|Struct|BreakCard_Data (.CardData (Utilities|Struct|BreakST_Card (LocalVariables|GetPlayerLaunchedCard))))) (.BaseSpeed (Utilities|Struct|BreakST_Character (LocalVariables|GetCharacterData)))) (+ (.ConsumedTime (Utilities|Struct|BreakCard_Data (.CardData (Utilities|Struct|BreakST_Card (LocalVariables|GetEnemyLaunchedCard))))) (.BaseSpeed (Utilities|Struct|BreakST_Enemy (LocalVariables|GetEnemyData)))))
        (Development|PrintString 0)
        (CallFunction|CardAction (LocalVariables|GetPlayerLaunchedCard) (LocalVariables|GetEnemyLaunchedCard) (LocalVariables|GetCharacterData) (LocalVariables|GetEnemyData) true)
        (else
          (Development|PrintString 0 "PRIMERO ENEMIGO")
          (CallFunction|CardAction (LocalVariables|GetPlayerLaunchedCard) (LocalVariables|GetEnemyLaunchedCard) (LocalVariables|GetCharacterData) (LocalVariables|GetEnemyData) false))))))

(fn CardAction
  (params (PlayerCard :type ST%20Card%20Structure) (EnemyCard :type ST%20Card%20Structure) (ChacarterData :type ST%20Character%20Structure) (EnemyData :type ST%20Enemy%20Structure) (PlayerFirst :type Boolean))
  (LocalVariables|SetLaunchedCard PlayerCard)
  (if PlayerFirst
    (bind _enemyoutput (CallFunction|PlayerHit PlayerCard EnemyCard ChacarterData EnemyData))
    (if (<= (.Life (Utilities|Struct|BreakST_Enemy _enemyoutput)) 0)
      (CallFunction|EnemyDead _enemyoutput)
      (else
        (bind _characteroutput (CallFunction|EnemyHit PlayerCard EnemyCard ChacarterData EnemyData))
        (if (<= (.Life (Utilities|Struct|BreakST_Character _characteroutput)) 0)
          (CallFunction|PlayerDead)
          (else
            (CallFunction|CardType (LocalVariables|GetLaunchedCard))
            (CallFunction|CardFate (LocalVariables|GetLaunchedCard))))))
    (else
      (bind _characteroutput_2 (CallFunction|EnemyHit PlayerCard EnemyCard ChacarterData EnemyData))
      (if (<= (.Life (Utilities|Struct|BreakST_Character _characteroutput_2)) 0)
        (CallFunction|PlayerDead)
        (else
          (bind _enemyoutput_2 (CallFunction|PlayerHit PlayerCard EnemyCard ChacarterData EnemyData))
          (if (<= (.Life (Utilities|Struct|BreakST_Enemy _enemyoutput_2)) 0)
            (CallFunction|EnemyDead _enemyoutput_2)
            (else
              (CallFunction|CardType (LocalVariables|GetLaunchedCard))
              (CallFunction|CardFate (LocalVariables|GetLaunchedCard)))))))))

(fn PlayerHit
  (params (PlayerCard :type ST%20Card%20Structure) (EnemyCard :type ST%20Card%20Structure) (CharacterData :type ST%20Character%20Structure) (EnemyData :type ST%20Enemy%20Structure))
  (bind _structout (Utilities|Struct|SetmembersinST_Enemy EnemyData (- (.Life (Utilities|Struct|BreakST_Enemy EnemyData)) (.BaseDamage (Utilities|Struct|BreakST_Character CharacterData)))))
  (bind _output_get (Variables|/Game/DarkMemoireProject/Blueprints/PlayerCharacter/Player.Player_C|SetEnemyData (.AsPlayer (Utilities|Casting|CastToPlayer (Game|GetPlayerCharacter 0))) _structout))
  (return _output_get))

(fn EnemyHit
  (params (PlayerCard :type ST%20Card%20Structure) (EnemyCard :type ST%20Card%20Structure) (CharacterData :type ST%20Character%20Structure) (EnemyData :type ST%20Enemy%20Structure))
  (bind _structout (Utilities|Struct|SetmembersinST_Character CharacterData (- (.Life (Utilities|Struct|BreakST_Character CharacterData)) (.BaseDamage (Utilities|Struct|BreakST_Enemy EnemyData)))))
  (bind _output_get (Variables|/Game/DarkMemoireProject/Blueprints/PlayerCharacter/Player.Player_C|SetCharacter%20Data (.AsPlayer (Utilities|Casting|CastToPlayer (Game|GetPlayerCharacter 0))) _structout))
  (return _output_get))

(fn EnemyDead
  (params (EnemyData :type ST%20Enemy%20Structure)))

(fn PlayerDead)

(fn CardType
  (params (CardType :type ST%20Card%20Structure))
  (bind _carddata (Utilities|Struct|BreakST_Card CardType))
  (bind (_cardtype _cardfate _cardeffect _consumedtime _consumedenergy _consumedsanity _usages) (Utilities|Struct|BreakCard_Data _carddata))
  (switch Utilities|FlowControl|Switch|SwitchonECardType _cardtype
    (:NewEnumerator3
      (bind _result (Math|Integer|DecrementInt _usages)
        (:%20%20
          (bind _structout (Utilities|Struct|SetmembersinCard_Data _carddata _result))
          (if (== (.Usages (Utilities|Struct|BreakCard_Data _structout)) 0)
            (bind _ascustom_game_instance (Utilities|Casting|CastToCustomGameInstance (Game|GetGameInstance)))
            (Utilities|Array|RemoveItem (Variables|/Game/DarkMemoireProject/DataManagement/GameData/CustomGameInstance.CustomGameInstance_C|GetCards _ascustom_game_instance) (.CardEffect (Utilities|Struct|BreakCard_Data _structout)))))))))

(fn CardFate
  (params (CardFate :type ST%20Card%20Structure))
  (switch Utilities|FlowControl|Switch|SwitchonECardFate (.CardFate (Utilities|Struct|BreakCard_Data (.CardData (Utilities|Struct|BreakST_Card CardFate))))))