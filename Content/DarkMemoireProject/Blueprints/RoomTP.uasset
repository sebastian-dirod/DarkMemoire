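; RoomTP is a room-transition trigger that teleports the player to the location of its linked Destiny actor.
; When a Player-tagged actor overlaps its collision box, it fires a dispatcher, locks movement and rotation, opens the door and shows a fade widget.
; Short delays time the relocation to the fade before control returns.
; Instances flagged IsDestiny ignore overlaps, so they do not trigger teleports.
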(event OnComponentBeginOverlap(CollisionBox)
  (params (OverlappedComponent :type Primitive%20Component%20Object%20Reference) (OtherActor :type Actor%20Object%20Reference) (OtherComp :type Primitive%20Component%20Object%20Reference) (OtherBodyIndex :type Integer) (bFromSweep :type Boolean) (SweepResult :type Hit%20Result%20Structure%20%28by%20ref%29))
  (if (Actor|ActorHasTag OtherActor "Player")
    (if (not (Variables|Default|GetIsDestiny))
      (Default|CallOnBeginOverlapDispatcher)
      (Default|ToggleMovementRotation (.AsPlayer (Utilities|Casting|CastToPlayer (Game|GetPlayerCharacter 0))) false false)
      (Default|OpenDoor (Variables|Default|GetDoor))
      (bind _returnvalue (UserInterface|CreateWidget "/Game/DarkMemoireProject/UMG/Generic/Fades.Fades_C"))
      (bind _output_get (Variables|Default|SetFade _returnvalue))
      (Variables|/Game/DarkMemoireProject/UMG/Generic/Fades.Fades_C|SetPlayAnim _output_get (Variables|/Game/DarkMemoireProject/UMG/Generic/Fades.Fades_C|GetFastFadeInOut _output_get))
      (Variables|/Game/DarkMemoireProject/UMG/Generic/Fades.Fades_C|SetDelayAnim _output_get 1.5)
      (UserInterface|Viewport|AddtoViewport _output_get 0)
      (Utilities|FlowControl|Delay 0.7)
      (Transformation|SetActorLocation (.AsPlayer (Utilities|Casting|CastToPlayer (Game|GetPlayerCharacter 0))) (Transformation|GetWorldLocation (Variables|RoomTP_C|GetDefaultSceneRoot (Variables|Default|GetDestiny))) false false)
      (Utilities|FlowControl|Delay 0.3)
      (Default|ToggleMovementRotation (.AsPlayer (Utilities|Casting|CastToPlayer (Game|GetPlayerCharacter 0))) true true))))

(fn ConstructionScript)